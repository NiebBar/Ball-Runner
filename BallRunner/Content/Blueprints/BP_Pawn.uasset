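; Pawn that moves its static mesh by applying torque from player axis input, likely as a rolling body.
; The left/right and forward/backward axis events share one Add Torque node, which feeds negatively scaled axis values into X and Y as an acceleration change, ignoring mass.
; A float-to-vector helper function and its macro are leftover scaffolding that never runs, and the other events are empty.
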(event `InputAxis|Move Left/Right`
  (params (AxisValue :type "Float (single-precision)"))
  (`PrimitiveComponent.AddTorqueInRadians` (`self.StaticMesh`) (`KismetMathLibrary.MakeVector` (* AxisValue -15.0) (* (stale `InputAxis|MoveForward/Backward` AxisValue) -15.0)) "None" true :!label _label))

(event `InputAxis|MoveForward/Backward`
  (params (AxisValue :type "Float (single-precision)"))
  (goto _label))

(fn `NewFunction_0`
  (params (InFloat :type "Float (double-precision)"))
  (returns (ReturnValue :type "Vector Structure"))
  (return (`KismetMathLibrary.Conv_DoubleToVector` InFloat)))

(fn `UserConstructionScript`)